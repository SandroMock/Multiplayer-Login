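; Game mode that tracks connected player controllers and spawns a third-person character for each joining player.
; Login and controller swaps add to the controller list, while logout removes exiting framework controllers.
; Spawning destroys any pawn already controlled, then possesses a new character at a random PlayerStart.
; After each login spawn, it calls SERVERSetName on all characters of player 0's class to refresh names.
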(event EventBeginPlay)

(event EventTick
  (params (DeltaSeconds :type Float%20%28single-precision%29)))

(event EventPostLogin
  (params (NewPlayer :type Player%20Controller%20Object%20Reference))
  ;[1 1 1] Event Connect
  (Utilities|Array|Add (Variables|Default|GetAll%20PCs) NewPlayer)
  (CallFunction|SpawnPlayer NewPlayer)
  (bind _asbp_third_person_character (Utilities|Casting|CastToBP_ThirdPersonCharacter (Game|GetPlayerCharacter 0)))
  (bind _outactors (Actor|GetAllActorsOfClass (Utilities|GetClass _asbp_third_person_character)))
  (for _array_element _outactors
    (Default|SERVERSetName _array_element)))

(event EventOnSwapPlayerControllers
  (params (OldPC :type Player%20Controller%20Object%20Reference) (NewPC :type Player%20Controller%20Object%20Reference))
  ;[1 1 1] Event Connect
  (Utilities|Array|Add (Variables|Default|GetAll%20PCs) NewPC))

(event EventOnLogout
  (params (ExitingController :type Controller%20Object%20Reference))
  ;[1 1 1] Event Disconnect
  (bind _asbp_pc_framework (Utilities|Casting|CastToBP_PC_Framework ExitingController))
  (Utilities|Array|RemoveItem (Variables|Default|GetAll%20PCs) _asbp_pc_framework))

(fn ConstructionScript)

(fn FindPlayerStart
  (bind _outactors (Actor|GetAllActorsOfClass "/Script/Engine.PlayerStart"))
  (return (Transformation|GetActorTransform (Utilities|Array|Get(acopy) _outactors (Math|Random|RandomIntegerinRange 0 (- (Utilities|Array|Length _outactors) 1))))))

(fn SpawnPlayer
  (params (Player%20Controller :type Player%20Controller%20Object%20Reference))
  (bind _returnvalue (Pawn|GetControlledPawn Player%20Controller))
  (Utilities|IsValid _returnvalue
    (:Is%20Valid
      (Actor|DestroyActor _returnvalue))
    (:Is%20Not%20Valid
      _))
  (bind _returnvalue_2 (Game|SpawnActorfromClass "/Game/ThirdPerson/Blueprints/BP_ThirdPersonCharacter.BP_ThirdPersonCharacter_C" (CallFunction|FindPlayerStart) "Undefined" 0 0))
  (Pawn|Possess Player%20Controller _returnvalue_2))